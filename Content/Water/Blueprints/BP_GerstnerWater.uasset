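; Base Blueprint for Gerstner-wave water that builds a grid of static mesh tiles and computes wave offsets and normals on the CPU, mirroring the material math.
; Construction spawns the centered tiles with an optional shared dynamic material instance.
; Child Blueprints override empty hooks for parameter setup, wave sampling and material settings.
; Height queries iteratively cancel horizontal wave displacement to approximate height at a requested location, with optional debug drawing.
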(event `self.ReceiveBeginPlay`
  (`self.InitiateGerstnerParameters`))

(fn `ComputeGerstnerWave`
  (params (Location :type "Vector Structure (by ref)") (Direction :type "Vector2D Structure (by ref)") (Wavelength :type "Float (double-precision)") (Amplitude :type "Float (double-precision)") (Steepness :type "Float (double-precision)") (ComputeNormal :type Boolean) (Time :type "Float (double-precision)"))
  (returns (GerstnerWorldLocation :type "Vector Structure") (GerstnerWorldOffset :type "Vector Structure") (GerstnerWorldNormal :type "Vector Structure"))
  (locals (ThisGerstnerNormal :type "Vector Structure" :default (0.0 0.0 1.0)) (ThisWaveK :type "Float (double-precision)" :default 0.0) (ThisWaveKA :type "Float (double-precision)" :default 0.0) (ThisWaveQ :type "Float (double-precision)" :default 0.0) (ThisWaveTime :type "Float (double-precision)" :default 0.0) (ThisWaveVector :type "Vector2D Structure") (ThisWavePos :type "Float (double-precision)" :default 0.0) (ThisWaveSin :type "Float (double-precision)" :default 0.0) (ThisWaveCos :type "Float (double-precision)" :default 0.0) (ThisGerstnerOffset :type "Vector Structure" :default (0.0 0.0 0.0)))
  (bind _thisgerstneroffset (`local.ThisGerstnerOffset`))
  (bind (_x _y) (`KismetMathLibrary.BreakVector2D` (* (`local.Direction`) (* (`local.ThisWaveQ`) -1.0 (`local.ThisWaveSin`) (`local.Amplitude`)))))
  (bind (_x_2 _y_2) (`KismetMathLibrary.BreakVector2D` (* (`local.Direction`) (* (`local.ThisWaveSin`) (`local.ThisWaveKA`)))))
  ;[1 1 1] compute offset just like we do in materials
  (bind _output_get (set `local.ThisWaveK` (/ (* (`KismetMathLibrary.GetPI`) 2.0) (`local.Wavelength`))))
  (bind _output_get_2 (set `local.ThisWaveKA` (* _output_get (`local.Amplitude`))))
  (set `local.ThisWaveQ` (/ (`local.Steepness`) _output_get_2))
  (set `local.ThisWaveTime` (* (`KismetMathLibrary.Sqrt` (* (`local.ThisWaveK`) 981.0)) (`local.Time`)))
  (bind _output_get_3 (set `local.ThisWaveVector` (* (`local.Direction`) (`local.ThisWaveK`))))
  (bind _output_get_4 (set `local.ThisWavePos` (- (`KismetMathLibrary.DotProduct2D` _output_get_3 (`KismetMathLibrary.Conv_VectorToVector2D` (`local.Location`))) (`local.ThisWaveTime`))))
  (set `local.ThisWaveSin` (`KismetMathLibrary.Sin` _output_get_4))
  (set `local.ThisWaveCos` (`KismetMathLibrary.Cos` _output_get_4))
  (set `local.ThisGerstnerOffset` (`KismetMathLibrary.MakeVector` _x _y (* (`local.ThisWaveCos`) (`local.Amplitude`))))
  ;[1 1 1] compute normals just like we do in materials
  (if (`local.ComputeNormal`)
    ;;[1 1 1] z component still needs to be flipped but we do that once we added all waves together
    (set `local.ThisGerstnerNormal` (`KismetMathLibrary.MakeVector` _x_2 _y_2 (* (`local.ThisWaveCos`) (`local.Steepness`) (`KismetMathLibrary.FClamp` (/ (* (`local.Amplitude`) 50.0) (`local.Wavelength`)))))))
  (return (+ (`local.Location`) _thisgerstneroffset) _thisgerstneroffset (`local.ThisGerstnerNormal`)))

(fn `ConstructWaterMeshComponents`
  (locals (ThisMaterial :type "MaterialInterface Object Reference"))
  (bind _material (`self.Material`))
  (`|ExecutionSequence`
    (:`then_0`
      ;[1 1 1] we may want to create a single dynamic material instance for all grid meshes
      (`/Engine/EditorBlueprintResources/StandardMacros.IsValid` _material
        (:`Is Valid`
          (bind _returnvalue (`KismetMaterialLibrary.CreateDynamicMaterialInstance` _material))
          (set `local.ThisMaterial` _returnvalue)
          (`self.InitiateDynamicMaterialInstance` _returnvalue))
        (:`Is Not Valid`
          (set `local.ThisMaterial` _material))))
    (:`then_1`
      (`self.SpawnWaterMeshComponents` (`local.ThisMaterial`)))))

(fn `GetGerstnerWaves`
  (params (Location :type "Vector Structure (by ref)") (Waves :type Integer :default 6) (WavesLimit :type Integer) (bComputeNormal :type Boolean :default true) (Time :type "Float (double-precision)"))
  (returns (WorldOffset :type "Vector Structure") (WorldNormal :type "Vector Structure") (WorldLocation :type "Vector Structure"))
  (locals (ThisOffset :type "Vector Structure" :default (0.0 0.0 0.0)) (ThisNormal :type "Vector Structure" :default (0.0 0.0 0.0)) (ThisMaxWave :type Integer :default 0) (ThisSteepness :type "Float (double-precision)" :default 0.0) (ThisAmplitude :type "Float (double-precision)" :default 0.0) (ThisWavelength :type "Float (double-precision)" :default 0.0) (ThisSpeed :type "Float (double-precision)" :default 0.0) (ThisDirection :type "Vector2D Structure") (ThisAlpha :type "Float (double-precision)" :default 0.0))
  ;[1 1 1] meant to be overriden by child blueprints depending on the sampling technique child blueprint is meant to 'use'
  (return (0.0 0.0 0.0) (0.0 0.0 0.0) (0.0 0.0 0.0)))

(fn `GetGerstnerWavesHeight`
  (params (Location :type "Vector Structure (by ref)") (Iteration :type Integer :default 3) (Waves :type Integer :default 6) (WavesLimit :type Integer :default 6) (bComputeNormal :type Boolean) (bDrawDebug :type Boolean))
  (returns (Offset :type "Vector Structure") (Normal :type "Vector Structure"))
  (locals (ThisOffset :type "Vector Structure" :default (0.0 0.0 0.0)) (ThisNormal :type "Vector Structure" :default (0.0 0.0 0.0)) (ThisIndex :type Integer))
  (bind _thisindex (`local.ThisIndex`))
  (bind _returnvalue (`KismetMathLibrary.LinearColorLerp` (struct) (struct :`R` 1.0 :`G` 1.0 :`B` 1.0 :`A` 1.0) (`KismetMathLibrary.MultiplyMultiply_FloatFloat` (/ (`KismetMathLibrary.Conv_IntToDouble` _thisindex) (`KismetMathLibrary.Conv_IntToDouble` (`local.Iteration`))) 2.2)))
  ;[1 1 1] getting the height of a Gerstner wave at a precise location isn't mathematically possible because whatever height you get from sampling that wave is the height at a shifted XY coordinate, so it's not the height at the location you asked for. So we need to approximate the result using an iterative approach. First iteration, we sample the height at the asked location. That'll give us a height at a shifted location in XY. For the second iteration, we sample the height at the asked location MINUS the XY offset we got from the previous iteration and we rince & repeat. Each time we have a smaller and smaller XY offset and we'll tend to a height that is exactly the height at the asked location. 3/4 iterations is usually considered good enough
  (for _index (range Iteration)
    (set `local.ThisIndex` _index)
    (bind (_worldoffset _worldnormal _worldlocation) (`self.GetGerstnerWaves` (- (`local.Location`) (* (`local.ThisOffset`) (1.0 1.0 0.0))) (`local.Waves`) (`local.WavesLimit`) (`local.bComputeNormal`) (+ (`KismetSystemLibrary.GetGameTimeInSeconds`) 100.0)))
    (set `local.ThisOffset` _worldoffset)
    (bind _output_get (set `local.ThisNormal` _worldnormal))
    (if (`local.bDrawDebug`)
      (`KismetSystemLibrary.DrawDebugLine` _worldlocation (+ _worldlocation (* _output_get (`KismetMathLibrary.Conv_IntToDouble` (+ (* _thisindex 50) 50)))) _returnvalue 0.0 1.0)
      (`KismetSystemLibrary.DrawDebugPoint` _worldlocation 20.0 _returnvalue)))
  (return (`local.ThisOffset`) (`local.ThisNormal`)))

(fn `InitiateDynamicMaterialInstance`
  (params (Material :type "MaterialInstanceDynamic Object Reference"))
  ;[1 1 1] meant to be overriden by child blueprints so we may forward extra settings that those child blueprints may have to the material instance
)

(fn `InitiateGerstnerParameters`
  (locals (ThisWaveIndex :type Integer) (ThisBaseName :type String))
  ;[1 1 1] meant to be overriden by child blueprints depending on the technique this child blueprint is meant to 'use'
)

(fn `SpawnWaterMeshComponents`
  (params (Material :type "MaterialInterface Object Reference"))
  (locals (ThisExtent :type "Vector Structure"))
  (bind _returnvalue (- (`self.Grid`) 1))
  (bind _returnvalue_2 (* (`self.GridScale`) (`self.MeshSize`) 0.5))
  (bind _returnvalue_3 (`KismetMathLibrary.Conv_IntToDouble` _returnvalue))
  (`/Engine/EditorBlueprintResources/StandardMacros.IsValid` (`self.Mesh`)
    (:`Is Valid`
      (set `local.ThisExtent` (`KismetMathLibrary.MakeVector` _returnvalue_2 _returnvalue_2))
      ;[1 1 1] create grid
      (for _index (range (+ _returnvalue 1))
        (for _index_2 (range (+ _returnvalue 1))
          (bind _returnvalue_4 (`AddComponent|NODE_AddStaticMeshComponent-1` :`RelativeTransform` (`KismetMathLibrary.MakeTransform` (* (- (`KismetMathLibrary.MakeVector` (`KismetMathLibrary.Conv_IntToDouble` _index) (`KismetMathLibrary.Conv_IntToDouble` _index_2)) (* (`KismetMathLibrary.MakeVector` _returnvalue_3 _returnvalue_3) 0.5)) (* (`KismetMathLibrary.GetMaxElement` (`local.ThisExtent`)) 2.0)) (struct) (`KismetMathLibrary.Conv_DoubleToVector` (`self.GridScale`)))))
          (`StaticMeshComponent.SetStaticMesh` _returnvalue_4 (`self.Mesh`))
          (`PrimitiveComponent.SetMaterial` _returnvalue_4 0 (`local.Material`)))))))

(fn `UserConstructionScript`
  (locals (ThisExtent :type "Vector Structure") (NewLocalVar_0 :type " Structure"))
  (`self.InitiateGerstnerParameters`)
  (`self.ConstructWaterMeshComponents`))