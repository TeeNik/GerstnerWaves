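; Gerstner water Blueprint that procedurally generates waves from wind direction, spread and min/max wavelength, amplitude and steepness ranges.
; InitiateGerstnerParameters copies these settings to the MC_GerstnerWaves parameter collection.
; GetGerstnerWaves sums waves into offset, normal and location, mirroring the material math for height sampling.
; Each wave gets a deterministic pseudo-random direction blended with wind, while a distribution exponent shapes its interpolation across the ranges.
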(event `self.ReceiveBeginPlay`
  (`parent.ReceiveBeginPlay`))

(fn `GetGerstnerWaveParameters`
  (params (Location :type "Vector Structure") (WaveDirection :type "Vector Structure") (WaveAlpha :type "Float (double-precision)"))
  (returns (Direction :type "Vector2D Structure") (Length :type "Float (double-precision)") (Amplitude :type "Float (double-precision)") (Steepness :type "Float (double-precision)"))
  (bind _wavealpha (`local.WaveAlpha`))
  ;[1 1 1] lerp parameters the same way we do in materials
  (return (`KismetMathLibrary.Normal2D` (`KismetMathLibrary.Conv_VectorToVector2D` (`KismetMathLibrary.VLerp` (`self.WindDirection`) WaveDirection (`self.Spread`)))) (`KismetMathLibrary.Lerp` (`self.MaxWaveLength`) (`self.MinWaveLength`) _wavealpha) (`KismetMathLibrary.Lerp` (`self.MaxAmplitude`) (`self.MinAmplitude`) _wavealpha) (`KismetMathLibrary.Lerp` (`self.MaxSteepness`) (`self.MinSteepness`) _wavealpha)))

(fn `GetGerstnerWaves`
  (params (Location :type "Vector Structure (by ref)") (Waves :type Integer) (WavesLimit :type Integer) (bComputeNormal :type Boolean) (Time :type "Float (double-precision)"))
  (returns (WorldOffset :type "Vector Structure") (WorldNormal :type "Vector Structure") (WorldLocation :type "Vector Structure"))
  (locals (ThisOffset :type "Vector Structure") (ThisNormal :type "Vector Structure") (ThisAlpha :type "Float (double-precision)") (ThisRandY :type Integer) (ThisRandX :type Integer) (ThisMaxWave :type Integer))
  (bind _thisoffset (`local.ThisOffset`))
  (bind _output_get (set `local.ThisMaxWave` (- (`KismetMathLibrary.Min` Waves (`self.WaveCount`)) 1)))
  ;[1 1 1] arbitrary start prime numbers
  (set `local.ThisRandX` 10007)
  (set `local.ThisRandY` 802709)
  ;[1 1 1] for each wave we might process, get alpha value based on current wave & total amount of waves
  (for _index (range (+ (`KismetMathLibrary.Min` _output_get (- WavesLimit 1)) 1))
    (set `local.ThisAlpha` (`KismetMathLibrary.MultiplyMultiply_FloatFloat` (/ (`KismetMathLibrary.Conv_IntToDouble` _index) (`KismetMathLibrary.Conv_IntToDouble` (`self.WaveCount`))) (`self.WaveDistribution`)))
    ;[1 1 1] generate sequence of numbers that *look* random and derive *pseudo* random direction from them
    (set `local.ThisRandX` (+ (* (`local.ThisRandX`) 1103515245) 12345))
    (set `local.ThisRandY` (+ (* (`local.ThisRandY`) 1103515245) 12345))
    ;[1 1 1] sum up all waves
    (bind (_direction _length _amplitude _steepness) (`self.GetGerstnerWaveParameters` (`local.Location`) (`KismetMathLibrary.Conv_Vector2DToVector` (- (* (`KismetMathLibrary.MakeVector2D` (`KismetMathLibrary.Cos` (/ (`KismetMathLibrary.Conv_IntToDouble` (`local.ThisRandX`)) 801571.0)) (`KismetMathLibrary.Sin` (/ (`KismetMathLibrary.Conv_IntToDouble` (`local.ThisRandY`)) 10223.0))) 2.0) 1.0)) (`local.ThisAlpha`)))
    (bind (_gerstnerworldlocation _gerstnerworldoffset _gerstnerworldnormal) (`self.ComputeGerstnerWave` (`local.Location`) _direction _length _amplitude _steepness (`local.bComputeNormal`) (`local.Time`)))
    (set `local.ThisOffset` (+ (`local.ThisOffset`) _gerstnerworldoffset))
    (set `local.ThisNormal` (+ _gerstnerworldnormal (`local.ThisNormal`))))
  ;[1 1 1] flip final normal's z component just like we do in materials
  (set `local.ThisNormal` (`KismetMathLibrary.Normal` (`KismetMathLibrary.MakeVector` (.x (`local.ThisNormal`)) (.y (`local.ThisNormal`)) (- 1.0 (.z (`local.ThisNormal`))))))
  (return _thisoffset (`local.ThisNormal`) (+ _thisoffset (`local.Location`))))

(fn `InitiateGerstnerParameters`
  ;[1 1 1] update parameters in case we use the 'RandomAmountOfWaves' method of sampling the waves' height via our 'GetGerstnerWavesHeight' function
  (`parent.InitiateGerstnerParameters`)
  (`KismetMaterialLibrary.SetVectorParameterValue` "/Game/Materials/Collections/MC_GerstnerWaves.MC_GerstnerWaves" "WindDirection" (`KismetMathLibrary.Conv_VectorToLinearColor` (`self.WindDirection`)))
  (`KismetMaterialLibrary.SetScalarParameterValue` "/Game/Materials/Collections/MC_GerstnerWaves.MC_GerstnerWaves" "Spread" (`self.Spread`))
  (`KismetMaterialLibrary.SetScalarParameterValue` "/Game/Materials/Collections/MC_GerstnerWaves.MC_GerstnerWaves" "WaveCount" (`KismetMathLibrary.Conv_IntToDouble` (`self.WaveCount`)))
  (`KismetMaterialLibrary.SetScalarParameterValue` "/Game/Materials/Collections/MC_GerstnerWaves.MC_GerstnerWaves" "MaxAmplitude" (`self.MaxAmplitude`))
  (`KismetMaterialLibrary.SetScalarParameterValue` "/Game/Materials/Collections/MC_GerstnerWaves.MC_GerstnerWaves" "MinAmplitude" (`self.MinAmplitude`))
  (`KismetMaterialLibrary.SetScalarParameterValue` "/Game/Materials/Collections/MC_GerstnerWaves.MC_GerstnerWaves" "MaxSteepness" (`self.MaxSteepness`))
  (`KismetMaterialLibrary.SetScalarParameterValue` "/Game/Materials/Collections/MC_GerstnerWaves.MC_GerstnerWaves" "MinSteepness" (`self.MinSteepness`))
  (`KismetMaterialLibrary.SetScalarParameterValue` "/Game/Materials/Collections/MC_GerstnerWaves.MC_GerstnerWaves" "MaxWaveLength" (`self.MaxWaveLength`))
  (`KismetMaterialLibrary.SetScalarParameterValue` "/Game/Materials/Collections/MC_GerstnerWaves.MC_GerstnerWaves" "MinWaveLength" (`self.MinWaveLength`))
  (`KismetMaterialLibrary.SetScalarParameterValue` "/Game/Materials/Collections/MC_GerstnerWaves.MC_GerstnerWaves" "WaveDistribution" (`self.WaveDistribution`)))

(fn `UserConstructionScript`
  (`parent.UserConstructionScript`))