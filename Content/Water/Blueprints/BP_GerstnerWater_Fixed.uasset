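; Gerstner wave water Blueprint that defines waves for rendering and evaluates their summed offset and normal at a given location.
; Wave directions blend from wind toward each wave's own direction by Spread, rebuilt at construction and after randomization.
; GetGerstnerWaves sums waves on the CPU, flipping normal Z to match materials.
; InitiateGerstnerParameters uploads up to six waves to a material parameter collection, which a Niagara collection mirrors.
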(event `self.ReceiveBeginPlay`
  (`parent.ReceiveBeginPlay`))

(fn `GetGerstnerWaves`
  (params (Location :type "Vector Structure (by ref)") (Waves :type Integer) (WavesLimit :type Integer) (bComputeNormal :type Boolean) (Time :type "Float (double-precision)"))
  (returns (WorldOffset :type "Vector Structure") (WorldNormal :type "Vector Structure") (WorldLocation :type "Vector Structure"))
  (locals (ThisMaxWave :type Integer) (ThisOffset :type "Vector Structure") (ThisNormal :type "Vector Structure"))
  (bind _wavesdirection (`self.WavesDirection`))
  (bind _thisoffset (`local.ThisOffset`))
  (bind _waves (`self.Waves`))
  ;[1 1 1] loop through user specified waves (up to X waves)
  (bind _output_get (set `local.ThisMaxWave` (`KismetMathLibrary.Min` (- (`KismetMathLibrary.Min` Waves WavesLimit) 1) (`KismetArrayLibrary.Array_LastIndex` (`self.Waves`)))))
  (for _index (range (+ _output_get 1))
    (if (and (`KismetArrayLibrary.Array_IsValidIndex` _waves _index) (`KismetArrayLibrary.Array_IsValidIndex` _wavesdirection _index))
      (bind ((`Length_21_08894B1E40F7FDFAEC2844A91CDD3ADB` _length) (`Amplitude_22_FDD22AB2443BD91CF60B85994BD5900A` _amplitude) (`Steepness_24_FB1C302240A7DA395F1946A000E823C0` _steepness)) (break `/Game/Water/Blueprints/SBP_GerstnerWave` (`|GetArrayItem` _waves _index)))
      ;[1 1 1] sum up all waves
      (bind (_gerstnerworldlocation _gerstnerworldoffset _gerstnerworldnormal) (`self.ComputeGerstnerWave` (`local.Location`) (`|GetArrayItem` _wavesdirection _index) _length _amplitude _steepness (`local.bComputeNormal`) (`local.Time`)))
      (set `local.ThisOffset` (+ (`local.ThisOffset`) _gerstnerworldoffset))
      (set `local.ThisNormal` (+ _gerstnerworldnormal (`local.ThisNormal`)))))
  (set `local.ThisNormal` (`KismetMathLibrary.Normal` (`KismetMathLibrary.MakeVector` (.x (`local.ThisNormal`)) (.y (`local.ThisNormal`)) (- 1.0 (.z (`local.ThisNormal`))))))
  (return _thisoffset (`local.ThisNormal`) (+ _thisoffset (`local.Location`))))

(fn `InitiateGerstnerParameters`
  (locals (ThisWaveIndex :type Integer) (ThisBaseName :type String))
  (bind _waves (`self.Waves`))
  (bind _wavesdirection (`self.WavesDirection`))
  ;[1 1 1] upload wave parameters to a Material parameter collection. A Niagara parameter collection is SYNCED with that material parameter collection, so it'll automatically be updated as well
  (for _index (range (+ (`KismetMathLibrary.Min` (`KismetArrayLibrary.Array_LastIndex` _waves) 5) 1))
    (if (and (`KismetArrayLibrary.Array_IsValidIndex` _waves _index) (`KismetArrayLibrary.Array_IsValidIndex` _wavesdirection _index))
      (bind _output_get (set `local.ThisWaveIndex` _index))
      (bind _output_get_2 (set `local.ThisBaseName` (`KismetStringLibrary.Concat_StrStr` "Wave" (`KismetStringLibrary.Conv_IntToString` (+ _output_get 1)))))
      (bind (_x _y) (`KismetMathLibrary.BreakVector2D` (`|GetArrayItem` _wavesdirection _index)))
      (bind ((`Length_21_08894B1E40F7FDFAEC2844A91CDD3ADB` _length) (`Amplitude_22_FDD22AB2443BD91CF60B85994BD5900A` _amplitude) (`Steepness_24_FB1C302240A7DA395F1946A000E823C0` _steepness)) (break `/Game/Water/Blueprints/SBP_GerstnerWave` (`|GetArrayItem` _waves _index)))
      (`KismetMaterialLibrary.SetVectorParameterValue` "/Game/Materials/Collections/MC_GerstnerWaves.MC_GerstnerWaves" (`KismetStringLibrary.Conv_StringToName` (`KismetStringLibrary.Concat_StrStr` _output_get_2 "DirLen")) (`KismetMathLibrary.MakeColor` _x _y _length 0.0))
      (`KismetMaterialLibrary.SetVectorParameterValue` "/Game/Materials/Collections/MC_GerstnerWaves.MC_GerstnerWaves" (`KismetStringLibrary.Conv_StringToName` (`KismetStringLibrary.Concat_StrStr` _output_get_2 "AmpSteep")) (make `LinearColor` _amplitude _steepness)))))

(fn `LerpWavesDirection`
  (bind _spread (`self.Spread`))
  (bind (_x _y) (`KismetMathLibrary.BreakVector2D` (`self.WindDirection`)))
  (`KismetArrayLibrary.Array_Clear` (`self.WavesDirection`))
  (for _array_element (`self.Waves`)
    (bind (_x_2 _y_2) (`KismetMathLibrary.BreakVector2D` (`.Direction_25_B7D10FE64DDCE426CF12A5A9E6AC45B6` (break `/Game/Water/Blueprints/SBP_GerstnerWave` _array_element))))
    (`KismetArrayLibrary.Array_Add` (`self.WavesDirection`) (`KismetMathLibrary.Normal2D` (`KismetMathLibrary.MakeVector2D` (`KismetMathLibrary.Lerp` _x _x_2 _spread) (`KismetMathLibrary.Lerp` _y _y_2 _spread))))))

(fn `RandomizeWavesDirection`
  (locals (ThisWave :type "/Game/Water/Blueprints/SBP_GerstnerWave Structure"))
  (for (_array_element _array_index) (`self.Waves`)
    (bind _output_get (set `local.ThisWave` _array_element))
    (bind _structout (setmembers `/Game/Water/Blueprints/SBP_GerstnerWave` :`StructRef` _output_get :`Direction` (`KismetMathLibrary.Normal2D` (`KismetMathLibrary.MakeVector2D` (`KismetMathLibrary.RandomFloatInRange` -1.0 1.0) (`KismetMathLibrary.RandomFloatInRange` -1.0 1.0)))))
    (`KismetArrayLibrary.Array_Set` (`self.Waves`) _array_index _structout))
  (`self.LerpWavesDirection`)
  (`self.InitiateGerstnerParameters`))

(fn `UserConstructionScript`
  (`self.LerpWavesDirection`)
  (`parent.UserConstructionScript`))