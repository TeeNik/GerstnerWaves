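; Physics actor that fakes buoyancy on Gerstner wave water by applying forces to its Cube at a set of buoyancy points.
; A low-rate looping timer samples wave height and normal per point, using limited waves and iterations to cut Blueprint cost.
; Submerged points get depth-scaled lift plus a sideways push from the surface normal.
; Tick interpolates forces and locations between samples, trading accuracy for performance.
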(event `self.ReceiveBeginPlay`
  (`KismetSystemLibrary.K2_SetTimer` null "GetBuoyancyForces" (`self.BuoyancyTickRate`) true)
  (`self.InitiateBuoyancyForces`))

(event `self.ReceiveTick`
  (params (DeltaSeconds :type "Float (single-precision)"))
  (`self.ApplyBuoyancyForces` DeltaSeconds))

(fn `ApplyBuoyancyForces`
  (params (DeltaTime :type "Float (double-precision)"))
  (locals (ThisForce :type "Vector Structure") (ThisLocation :type "Vector Structure"))
  (bind _deltatime (`local.DeltaTime`))
  (bind _thisforce (`local.ThisForce`))
  ;[1 1 1] interpolate both forces and forces locations. We do this because sampling Gerstner Waves' Height for each of our buoyant points is very expensive so we do this every now and then and interpolate the result on tick instead. This results in a big approximation but works well enough!
  (for (_ _array_index) (`self.BuoyancyPoints`)
    (set `local.ThisLocation` (`KismetMathLibrary.VInterpTo` (`|GetArrayItem` (`self.BuoyancyForcesLocation`) _array_index) (`|GetArrayItem` (`self.BuoyancyTargetForcesLocation`) _array_index) _deltatime 20.0))
    (set `local.ThisForce` (`KismetMathLibrary.VInterpTo` (`|GetArrayItem` (`self.BuoyancyForces`) _array_index) (`|GetArrayItem` (`self.BuoyancyTargetForces`) _array_index) _deltatime 20.0))
    ;[1 1 1] update interpolated values
    (`KismetArrayLibrary.Array_Set` (`self.BuoyancyForces`) _array_index _thisforce true)
    (`KismetArrayLibrary.Array_Set` (`self.BuoyancyForcesLocation`) _array_index (`local.ThisLocation`) true)
    ;[1 1 1] add force if any to add. This can be quite unstable! Feel free to play with the 'Box' physics properties such as Linear & Angular drag & Center of Mass to make it stable
    (if (not (`KismetMathLibrary.Vector_IsZero` _thisforce))
      (`PrimitiveComponent.AddForceAtLocation` (`self.Cube`) (`local.ThisForce`) (`local.ThisLocation`) "None"))))

(fn `GetBuoyancyForces`
  (locals (ThisLocation :type "Vector Structure" :default (0.0 0.0 0.0)) (ThisBuoyancyLocation :type "Vector Structure" :default (0.0 0.0 0.0)) (ThisOffset :type "Vector Structure" :default (0.0 0.0 0.0)) (ThisNormal :type "Vector Structure" :default (0.0 0.0 0.0)) (ThisBuoyancyDelta :type "Float (double-precision)" :default 0.0) (ThisBuoyancyIndex :type Integer))
  (bind _buoyancytargetforces (`self.BuoyancyTargetForces`))
  (bind _thisbuoyancyindex (`local.ThisBuoyancyIndex`))
  (bind _buoyancysidewaysforce (`self.BuoyancySidewaysForce`))
  (`/Engine/EditorBlueprintResources/StandardMacros.IsValid` (`self.Water`)
    (:`Is Valid`
      ;[1 1 1] for each buoyant point, transform its location from location to world space
      (for (_array_element _array_index) (`self.BuoyancyPoints`)
        (set `local.ThisBuoyancyIndex` _array_index)
        (bind _output_get (set `local.ThisLocation` (`KismetMathLibrary.TransformLocation` (`self.GetTransform`) _array_element)))
        ;[1 1 1] do 2 iterations and limit to the first 3 waves (we hardcoded 6 Gerstner Waves and the last three are the smaller ones so they don't have that much impact on the water overall displacement so we can probably skip those and deal with some approximations in our 'fake' buoyancy). We do this for EACH buoyant point already so there's 3 embedded for loops and blueprints are at their worst when that happens so this is costly! This is why we limit both the iteration & wave amount and call this function with a low-rate timer!
        (bind (_offset _normal) (`/Game/Water/Blueprints/BP_GerstnerWater.GetGerstnerWavesHeight` (`self.Water`) _output_get 2 6 3 true false))
        (set `local.ThisOffset` _offset)
        (set `local.ThisNormal` _normal)
        ;[1 1 1] project buoyant point onto water surface and check the vertical delta with its original location
        (bind _output_get_2 (set `local.ThisBuoyancyLocation` (+ (`KismetMathLibrary.MakeVector` (.x (`local.ThisLocation`)) (.y (`local.ThisLocation`)) (.z (`self.K2_GetActorLocation` (`self.Water`)))) (`KismetMathLibrary.MakeVector` 0.0 0.0 (.z (`local.ThisOffset`))))))
        (`KismetArrayLibrary.Array_Set` (`self.BuoyancyTargetForcesLocation`) (`local.ThisBuoyancyIndex`) _output_get_2 true)
        (bind _output_get_3 (set `local.ThisBuoyancyDelta` (+ (.z (- _output_get_2 (`local.ThisLocation`))) (`self.BuoyancyVerticalOffset`))))
        (if (> _output_get_3 0.0)
          ;[1 1 1] push up depending on how deep in water we are & sideways depending on water normal
          (`KismetArrayLibrary.Array_Set` _buoyancytargetforces _thisbuoyancyindex (`KismetMathLibrary.MakeVector` (* (.x (`local.ThisNormal`)) _buoyancysidewaysforce 100.0) (* (.y (`local.ThisNormal`)) _buoyancysidewaysforce 100.0) (* (`KismetMathLibrary.FMin` (`KismetMathLibrary.FMax` (`local.ThisBuoyancyDelta`)) 100.0) (`self.BuoyancyVerticalForce`))) true)
          (else
            (`KismetArrayLibrary.Array_Set` _buoyancytargetforces _thisbuoyancyindex (0.0 0.0 0.0) true)))))
    (:`Is Not Valid`
      (`KismetSystemLibrary.K2_ClearTimer` null "GetBuoyancyForces"))))

(fn `InitiateBuoyancyForces`
  (`KismetArrayLibrary.Array_Clear` (`self.BuoyancyForcesLocation`))
  (for _array_element (`self.BuoyancyPoints`)
    (`KismetArrayLibrary.Array_Add` (`self.BuoyancyForcesLocation`) (`KismetMathLibrary.TransformLocation` (`self.GetTransform`) _array_element)))
  (`KismetArrayLibrary.Array_Set` (`self.BuoyancyForces`) (`KismetArrayLibrary.Array_LastIndex` (`self.BuoyancyPoints`)) (0.0 0.0 0.0) true)
  (set `self.BuoyancyTargetForces` (`self.BuoyancyForces`))
  (set `self.BuoyancyTargetForcesLocation` (`self.BuoyancyForcesLocation`)))

(fn `UserConstructionScript`)