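; Fake buoyancy Blueprint that makes a floating scene component bob and tilt on Gerstner wave water without physics.
; A looping timer samples wave offset and normal from the Water reference at the actor's location, stopping if that reference is invalid.
; Tick interpolates the component toward the cached height and a normal-aligned rotation, smoothing motion between samples.
; BeginPlay takes an initial sample and snaps the component to it.
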(event `self.ReceiveBeginPlay`
  (bind _normal (`self.Normal`))
  (bind _returnvalue (`KismetMathLibrary.Cross_VectorVector` (-1.0 0.0 0.0) _normal))
  (`KismetSystemLibrary.K2_SetTimer` null "SampleWater" (`self.SampleWaterRate`) true)
  (`self.SampleWater`)
  (`SceneComponent.K2_SetRelativeLocationAndRotation` (`self.FloatingScene`) (`self.Offset`) (`KismetMathLibrary.MakeRotationFromAxes` (`KismetMathLibrary.Cross_VectorVector` _returnvalue _normal) _returnvalue _normal) false false))

(event `self.ReceiveTick`
  (params (DeltaSeconds :type "Float (single-precision)"))
  (bind _normal (`self.Normal`))
  (bind _floatingscene (`self.FloatingScene`))
  (bind _returnvalue (`KismetMathLibrary.Cross_VectorVector` (-1.0 0.0 0.0) _normal))
  (`SceneComponent.K2_SetRelativeLocationAndRotation` _floatingscene (`KismetMathLibrary.VInterpTo` (`SceneComponent.RelativeLocation` _floatingscene) (`KismetMathLibrary.MakeVector` 0.0 0.0 (.z (`self.Offset`))) DeltaSeconds 10.0) (`KismetMathLibrary.RInterpTo` (`SceneComponent.K2_GetComponentRotation` _floatingscene) (`KismetMathLibrary.MakeRotationFromAxes` (`KismetMathLibrary.Cross_VectorVector` _returnvalue _normal) _returnvalue _normal) DeltaSeconds 10.0) false false))

(fn `SampleWater`
  (bind _water (`self.Water`))
  (`/Engine/EditorBlueprintResources/StandardMacros.IsValid` _water
    (:`Is Valid`
      (bind (_offset _normal) (`/Game/Water/Blueprints/BP_GerstnerWater.GetGerstnerWavesHeight` _water (`self.K2_GetActorLocation`) 3 6 6 true false))
      (set `self.Offset` _offset)
      (set `self.Normal` _normal))
    (:`Is Not Valid`
      (`KismetSystemLibrary.K2_ClearTimer` null "SampleWater"))))

(fn `UserConstructionScript`)